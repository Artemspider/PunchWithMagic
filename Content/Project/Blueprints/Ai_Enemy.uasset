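; Melee AI enemy that chases the player, throws random boxing attacks, and ragdolls when killed.
; An AIMoveTo loop picks one of three montages, whose notifies line-trace between attack points to apply damage.
; AnyDamage triggers the damage type's status effect, plays random hit reactions and reduces health; a looping timer reapplies the last damage as DOT.
; BeginPlay increments the GameMode's EnemiesLeft via misleadingly named EnemyDead; death decrements it.
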(event `StartDOT`
  ;[1 1 1] Damage Over Time
  (bind _returnvalue (`KismetSystemLibrary.K2_SetTimerDelegate` (delegate `DOT`) 1.0 true))
  (set `self.DOT Timer` _returnvalue))

(event `DOT`
  ;[1 1 1] Damage Over Time
  (`GameplayStatics.ApplyDamage` self (`self.Damage`)))

(event `EndDOT`
  ;[1 1 1] Damage Over Time
  (`KismetSystemLibrary.K2_ClearAndInvalidateTimerHandle` (`self.DOT Timer`)))

(event `self.ReceiveAnyDamage`
  (params (Damage :type "Float (single-precision)") (DamageType :type "DamageType Object Reference") (InstigatedBy :type "Controller Object Reference") (DamageCauser :type "Actor Object Reference"))
  (bind _returnvalue (`KismetMathLibrary.RandomIntegerInRange` 1 2))
  ;[1 1 1] Health
  (`GameplayStatics.PlaySound2D` "/Game/Project/sound/KEEPON_Voice_EnemyA_Death3.KEEPON_Voice_EnemyA_Death3" 1.0 1.0 0.0 null null)
  (set `self.Damage` Damage)
  (`KismetSystemLibrary.PrintString` "Ouch" true true (struct :`G` 0.66 :`B` 1.0 :`A` 1.0) 0.5)
  (message `/Game/Project/Blueprints/DamageTypeInterface.TriggerEffect` DamageType (`self.StatusEffectComponent`))
  (if (== _returnvalue 1) :!label _label
    (set `self.CanAttack` true)
    (`|PlayMontage` (`self.Mesh`) "/Game/Project/Animation/EnemyAnim/Head_Hit_Montage.Head_Hit_Montage"
      (:`then`
        _)
      (:`OnCompleted`
        (set `self.CanAttack` false :!label _label_2)))
    (elif (== _returnvalue 2)
      (set `self.CanAttack` true)
      (`|PlayMontage` (`self.Mesh`) "/Game/Project/Animation/EnemyAnim/Stomach_Hit_Montage.Stomach_Hit_Montage"
        (:`then`
          _)
        (:`OnCompleted`
          (goto _label_2)))
      (else
        (goto _label))))
  (if (<= 0.0 (`self.NPCHealth`))
    (set `self.NPCHealth` (- (`self.NPCHealth`) (`self.Damage`)))
    (else
      (`GameplayStatics.PlaySound2D` "/Game/Project/sound/KEEPON_Voice_EnemyB_Death1.KEEPON_Voice_EnemyB_Death1" 1.0 1.0 0.0 null null)
      (set `self.CanAttack` true)
      (`PrimitiveComponent.SetSimulatePhysics` (`self.Mesh`) true)
      (bind _asbp_third_person_game_mode (cast `/Game/Project/Blueprints/BP_ThirdPersonGameMode` (`GameplayStatics.GetGameMode`)))
      (set `/Game/Project/Blueprints/BP_ThirdPersonGameMode.EnemiesLeft` (- (`/Game/Project/Blueprints/BP_ThirdPersonGameMode.EnemiesLeft` _asbp_third_person_game_mode) 1) _asbp_third_person_game_mode)
      (`ActorComponent.K2_DestroyComponent` (`self.CapsuleComponent`)))))

(event `FollowPlayer`
  (bind _returnvalue (`KismetMathLibrary.RandomIntegerInRange` 1 3))
  ;[1 1 1] AI and Attacks
  (`|AIMoveTo` self (0.0 0.0 0.0) (`GameplayStatics.GetPlayerCharacter` 0) 100.0
    (:`OnSuccess`
      (if (== _returnvalue 1) :!label _label_3
        (`KismetSystemLibrary.Delay` 0.55)
        (set `self.CanAttack` true)
        (`|PlayMontage` (`self.Mesh`) "/Game/Project/Animation/EnemyAnim/Boxing_Montage.Boxing_Montage"
          (:`OnCompleted`
            (`KismetSystemLibrary.Delay` 1.5 :!label _label_4))
          (:`OnInterrupted`
            _)
          (:`OnNotifyBegin`
            (bind _outhit (`KismetSystemLibrary.LineTraceSingle` :`Start` (`SceneComponent.GetSocketLocation` (`self.AttackStart`) "None") :`End` (`SceneComponent.GetSocketLocation` (`self.AttackEnd`) "None") :`TraceChannel` "TraceTypeQuery1" :`DrawDebugType` "ForDuration" :`DrawTime` 0.5 :!label _label_5))
            (`GameplayStatics.ApplyDamage` (`.HitActor` (`GameplayStatics.BreakHitResult` _outhit)) 10.0 null self)
            (goto _label_4)))
        (elif (== _returnvalue 2)
          (`KismetSystemLibrary.Delay` 0.65)
          (set `self.CanAttack` true)
          (`|PlayMontage` (`self.Mesh`) "/Game/Project/Animation/EnemyAnim/Boxing__1__Montage.Boxing__1__Montage"
            (:`OnCompleted`
              (goto _label_4))
            (:`OnInterrupted`
              _)
            (:`OnNotifyBegin`
              (goto _label_5)))
          (elif (== _returnvalue 3)
            (`KismetSystemLibrary.Delay` 0.75)
            (set `self.CanAttack` true)
            (`|PlayMontage` (`self.Mesh`) "/Game/Project/Animation/EnemyAnim/Boxing__2__Montage.Boxing__2__Montage"
              (:`OnCompleted`
                (goto _label_4))
              (:`OnInterrupted`
                _)
              (:`OnNotifyBegin`
                (goto _label_5)))
            (else
              (goto _label_3)))))
      (set `self.CanAttack` false)
      (`KismetSystemLibrary.Delay` 0.5)
      (`self.FollowPlayer`))
    (:`OnFail`
      (set `self.CanAttack` false)
      (`KismetSystemLibrary.Delay` 0.5)
      (`self.FollowPlayer`))))

(event `self.ReceiveBeginPlay`
  ;[1 1 1] AI and Attacks
  (`|ExecutionSequence`
    (:`then_0`
      (if (not (`self.CanAttack`))
        (`self.FollowPlayer`)))
    (:`then_1`
      (`self.EnemyDead`))))

(event `EnemyDead`
  ;[1 1 1] AI and Attacks
  (bind _asbp_third_person_game_mode (cast `/Game/Project/Blueprints/BP_ThirdPersonGameMode` (`GameplayStatics.GetGameMode`)))
  (set `/Game/Project/Blueprints/BP_ThirdPersonGameMode.EnemiesLeft` (+ (`/Game/Project/Blueprints/BP_ThirdPersonGameMode.EnemiesLeft` _asbp_third_person_game_mode) 1) _asbp_third_person_game_mode))

(fn `EnemyREF`
  (returns (EnemyREF :type "/Game/Project/Blueprints/Enemy_AI Object Reference"))
  (return self))

(fn `UserConstructionScript`)
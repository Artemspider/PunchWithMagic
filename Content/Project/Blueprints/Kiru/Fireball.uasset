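; Fireball projectile, apparently Kiru's, that deals fire damage and reports it back as restorable health.
; On sphere hit it plays a sound, fires OnProjectImpact, then line-traces between its start and end components, with debug drawing, to choose the damaged actor.
; It passes the trace result and damage dealt to Kiru_Blueprint's RestoreHealthMessage, spawns a reversed-yaw explosion and destroys itself.
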(event `self.Sphere.OnComponentHit`
  (params (HitComponent :type "PrimitiveComponent Object Reference") (OtherActor :type "Actor Object Reference") (OtherComp :type "PrimitiveComponent Object Reference") (NormalImpulse :type "Vector Structure") (Hit :type "HitResult Structure (by ref)"))
  (bind (_returnvalue_roll _returnvalue_pitch _returnvalue_yaw) (`KismetMathLibrary.BreakRotator` (`self.K2_GetActorRotation`)))
  (`GameplayStatics.PlaySound2D` "/Game/Project/sound/KEEPON_Fball_Hit1.KEEPON_Fball_Hit1" 1.0 1.0 0.0 null null)
  (`self.OnProjectImpact` OtherActor Hit)
  (bind (_outhit _returnvalue) (`KismetSystemLibrary.LineTraceSingle` :`Start` (`SceneComponent.GetSocketLocation` (`self.FireballStart`) "None") :`End` (`SceneComponent.GetSocketLocation` (`self.FireballEnd`) "None") :`TraceChannel` "TraceTypeQuery1" :`DrawDebugType` "ForDuration" :`DrawTime` 0.5))
  (bind _returnvalue_2 (`GameplayStatics.ApplyDamage` (`.HitActor` (`GameplayStatics.BreakHitResult` _outhit)) 20.0 null null "/Game/Project/Blueprints/Kiru/Fire.Fire_C"))
  (bind _returnvalue_3 (`GameplayStatics.GetActorOfClass` "/Game/Project/Blueprints/Kiru/Kiru_Blueprint.Kiru_Blueprint_C"))
  (message `/Game/Project/Blueprints/Kiru/BPI_RestoreHealth.RestoreHealth` _returnvalue_3 _returnvalue _returnvalue_2)
  (`GameplayStatics.SpawnEmitterAtLocation` "/Game/Project/Realistic_Starter_VFX_Pack_Vol2/Particles/Explosion/P_Explosion_Side.P_Explosion_Side" (`self.K2_GetActorLocation`) (`KismetMathLibrary.MakeRotator` _returnvalue_roll _returnvalue_pitch (+ _returnvalue_yaw 180.0)))
  (`KismetSystemLibrary.Delay` 0.0)
  (`self.K2_DestroyActor`))

(fn `NewFunction`)

(fn `UserConstructionScript`)
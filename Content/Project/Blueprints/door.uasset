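; Door Blueprint that swings open when its trigger is overlapped and no enemies are left.
; On overlap it reads EnemiesLeft from BP_ThirdPersonGameMode; despite its name, EnemiesAreAlive is true when that count is zero.
; A timeline drives the yaw of the Rot component to open the door, then reverses one second after overlap ends.
; The overlap events do not filter which actor triggers them.
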(event `self.ReceiveBeginPlay`)

(event `Open Door`
  (bind _asbp_third_person_game_mode (cast `/Game/Project/Blueprints/BP_ThirdPersonGameMode` (`GameplayStatics.GetGameMode`)))
  (set `self.EnemiesAreAlive?` (== (`/Game/Project/Blueprints/BP_ThirdPersonGameMode.EnemiesLeft` _asbp_third_person_game_mode) 0)))

(event `OD`
  (bind (_direction _newtrack_0) (`Timeline|Timeline` :!label _label)
    (:`Update`
      (`SceneComponent.K2_SetRelativeRotation` (`self.rot`) (`KismetMathLibrary.MakeRotator` 0.0 0.0 _newtrack_0) false false))))

(event `self.trigger.OnComponentBeginOverlap`
  (params (OverlappedComponent :type "PrimitiveComponent Object Reference") (OtherActor :type "Actor Object Reference") (OtherComp :type "PrimitiveComponent Object Reference") (OtherBodyIndex :type Integer) (bFromSweep :type Boolean) (SweepResult :type "HitResult Structure (by ref)"))
  (`self.Open Door`)
  (if (`self.EnemiesAreAlive?`)
    (`self.OD`)))

(event `self.trigger.OnComponentEndOverlap`
  (params (OverlappedComponent :type "PrimitiveComponent Object Reference") (OtherActor :type "Actor Object Reference") (OtherComp :type "PrimitiveComponent Object Reference") (OtherBodyIndex :type Integer))
  (set `self.TriggerIsOverlaped` false)
  (`KismetSystemLibrary.Delay` 1.0)
  (goto _label :!via `Reverse`))

(fn `UserConstructionScript`)
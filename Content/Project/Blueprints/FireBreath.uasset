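; FireBreath is an attack volume that applies damage over time to enemies overlapping its sphere and restores health to Kiru.
; On overlap begin it gets the enemy through an EnemyREFMessage call, sets its damage and starts its DOT.
; It then finds Kiru_Blueprint by class and sends a fireball-hit heal equal to that damage, once per overlap.
; Overlap end stops the enemy's DOT.
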(event `self.Sphere.OnComponentBeginOverlap`
  (params (OverlappedComponent :type "PrimitiveComponent Object Reference") (OtherActor :type "Actor Object Reference") (OtherComp :type "PrimitiveComponent Object Reference") (OtherBodyIndex :type Integer) (bFromSweep :type Boolean) (SweepResult :type "HitResult Structure (by ref)"))
  (bind _enemyref (message `/Game/Project/Blueprints/EnemyReference.EnemyREF` OtherActor))
  (`/Engine/EditorBlueprintResources/StandardMacros.IsValid` _enemyref
    (:`Is Valid`
      (bind _output_get (set `/Game/Project/Blueprints/Enemy/AI_Enemy.Damage` 1.0 _enemyref))
      (`/Game/Project/Blueprints/Enemy/AI_Enemy.Dot` _enemyref)
      (`/Game/Project/Blueprints/Enemy/AI_Enemy.StartDOT` _enemyref)
      (bind _returnvalue (`GameplayStatics.GetActorOfClass` "/Game/Project/Blueprints/Kiru_Blueprint.Kiru_Blueprint_C"))
      (message `/Game/Project/Blueprints/BPI_RestoreHealth.RestoreHealth` _returnvalue true _output_get))))

(event `self.Sphere.OnComponentEndOverlap`
  (params (OverlappedComponent :type "PrimitiveComponent Object Reference") (OtherActor :type "Actor Object Reference") (OtherComp :type "PrimitiveComponent Object Reference") (OtherBodyIndex :type Integer))
  (bind _enemyref (message `/Game/Project/Blueprints/EnemyReference.EnemyREF` OtherActor))
  (`/Engine/EditorBlueprintResources/StandardMacros.IsValid` _enemyref
    (:`Is Valid`
      (`/Game/Project/Blueprints/Enemy/AI_Enemy.EndDOT` _enemyref))))

(fn `UserConstructionScript`)